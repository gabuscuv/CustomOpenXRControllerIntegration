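; OpenXR controller actor that displays a left or right mesh matching the detected VR controller, with button highlighting.
; On BeginPlay it polls for the controller type until found, unless spoofing is enabled, which overrides the type outside distribution builds.
; SetMesh picks mesh and material by device and system-name substrings, offsetting it when a child actor.
; Highlights toggle material scalar parameters named after button enums; Trigger and Grip can also shift the mesh.
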(event `self.ReceiveBeginPlay`
  (bind (_trackingsystemname _devicetype) (`OpenXRExpansionFunctionLibrary.GetXRMotionControllerType` :!label _label)
    (:`OnSucceeded`
      _)
    (:`OnFailed`
      (if (`self.SpoofController`)
        _
        (else
          (`KismetSystemLibrary.Delay` 0.5)
          (goto _label)))))
  (bind (_returnvalue _returnvalue2) (`self.SpoofingControllers` _trackingsystemname _devicetype))
  (`self.SetMesh` _returnvalue _returnvalue2))

(event `self.HighlightActionButton`
  (params (Button :type Byte) (Enable :type Boolean) (AddOffset :type Boolean))
  (bind _base (`self.Base`))
  (switch `/CustomOpenXRControllerIntegration/Enums/EButtons` "NewEnumerator0"
    (:`NewEnumerator0`
      _)
    (:`NewEnumerator1`
      _)
    (:`NewEnumerator5`
      _)
    (:`NewEnumerator2`
      _)
    (:`NewEnumerator3`
      (if (and Enable AddOffset) :!label _label_2
        (`SceneComponent.K2_AddRelativeLocation` _base (0.0 0.0 10.0) false false)
        (else
          (`SceneComponent.K2_SetRelativeLocation` _base (`self.DefaultVector`) false false))))
    (:`NewEnumerator4`
      (goto _label_2))
    (:`NewEnumerator6`
      _)
    (:`NewEnumerator7`
      _)
    (:`NewEnumerator8`
      _)
    (:`NewEnumerator9`
      _)
    (:`NewEnumerator10`
      _))
  (`self.HighlightButtons` (cast `/CustomOpenXRControllerIntegration/Enums/EButtons` Button) Enable))

(event `self.ClearAllButtons`
  (bind _enumvalue (foreach `/CustomOpenXRControllerIntegration/Enums/EButtons` false)
    (:`LoopBody`
      (`self.HighlightButtons` _enumvalue)
      (`SceneComponent.K2_SetRelativeLocation` (`self.Base`) (`self.DefaultVector`) false false))))

(fn `HighlightButtons`
  (params (Enumerator :type "/CustomOpenXRControllerIntegration/Enums/EButtons Enum" :default "NewEnumerator0") (A :type Boolean))
  (`MeshComponent.SetScalarParameterValueOnMaterials` (`self.Base`) (`KismetStringLibrary.Conv_StringToName` (`|GetEnumeratorNameAsString` Enumerator)) (`KismetMathLibrary.Conv_BoolToDouble` (not A))))

(fn `isOculusTouchv2`
  (params (SearchIn :type String))
  (returns (ReturnValue :type Boolean))
  (return (or (`KismetStringLibrary.Contains` SearchIn "Quest 1" false true) (`KismetStringLibrary.Contains` SearchIn "Rift S" false true))))

(fn `SetMesh`
  (params (InputPin :type "EBPOpenXRControllerDeviceType Enum" :default "DT_SimpleController") (InputPin2 :type String))
  (bind _base (`self.Base`))
  (bind _base_2 (`self.Base`))
  (bind _base_3 (`self.Base`))
  (bind _base_4 (`self.Base`))
  (bind _base_5 (`self.Base`))
  (bind _base_6 (`self.Base`))
  (bind _base_7 (`self.Base`))
  (bind _base_8 (`self.Base`))
  (if (`self.Left`)
    (switch `EBPOpenXRControllerDeviceType` InputPin
      (:`DT_ValveIndexController`
        (`StaticMeshComponent.SetStaticMesh` (`self.Base`) "/OpenXR/Devices/ValveIndex/Left/left_ValveIndexController.left_ValveIndexController")
        (`PrimitiveComponent.CreateDynamicMaterialInstance` (`self.Base`) 0 "/CustomOpenXRControllerIntegration/Materials/ValveIndex/MI_XRController_ValveIndex_Left.MI_XRController_ValveIndex_Left" "None")
        (`self.isChild Actor`
          (:`true`
            (`SceneComponent.K2_SetRelativeLocation` _base_8 (-5.0 2.0 -2.0) false true))))
      (:`DT_ViveController`
        (`StaticMeshComponent.SetStaticMesh` _base_8 "/OpenXR/Devices/HTCVive/HTCViveController.HTCViveController" :!label _label)
        (`self.isChild Actor` :!label _label_2
          (:`true`
            (`SceneComponent.K2_SetRelativeLocation` _base_7 (-5.0 4.0 -2.0) false true))))
      (:`DT_ViveProController`
        (goto _label))
      (:`DT_OculusTouchController`
        (`self.GetOculusTouchVersion` InputPin2 :!label _label_3
          (:`Oculus Touch V2`
            (`StaticMeshComponent.SetStaticMesh` (`self.Base`) "/OpenXR/Devices/OculusTouch_v2/Left/left_OculusTouch_v2Controller.left_OculusTouch_v2Controller")
            (`PrimitiveComponent.CreateDynamicMaterialInstance` (`self.Base`) 0 "/CustomOpenXRControllerIntegration/Materials/OculusTouch_v2/MI_XRController_OculusTouch_v2_Left.MI_XRController_OculusTouch_v2_Left" "None")
            (`self.isChild Actor` :!label _label_4
              (:`true`
                (`SceneComponent.K2_SetRelativeLocation` _base_3 (-5.0 5.0 0.0) false true))))
          (:`Oculus Touch V3`
            (`StaticMeshComponent.SetStaticMesh` _base_4 "/OpenXR/Devices/OculusTouch_v3/Left/left_OculusTouch_v3Controller.left_OculusTouch_v3Controller")
            (`PrimitiveComponent.CreateDynamicMaterialInstance` (`self.Base`) 0 "/CustomOpenXRControllerIntegration/Materials/OculusTouch_v3/MI_XRController_OculusTouch_v3_Left.MI_XRController_OculusTouch_v3_Left" "None")
            (goto _label_4))
          (:`Oculus Touch V1`
            (`StaticMeshComponent.SetStaticMesh` _base_4 "/OpenXR/Devices/OculusTouch/Left/left_OculusTouchController.left_OculusTouchController")
            (`PrimitiveComponent.CreateDynamicMaterialInstance` (`self.Base`) 0 "/CustomOpenXRControllerIntegration/Materials/OculusTouch/MI_XRController_OculusTouch_Left.MI_XRController_OculusTouch_Left" "None")
            (`self.isChild Actor`
              (:`true`
                (`SceneComponent.K2_SetRelativeLocation` _base_3 (-5.0 5.0 -2.0) false true))))))
      (:`DT_MicrosoftMotionController`
        (if (`KismetStringLibrary.Contains` InputPin2 "Reverb G2")
          (`StaticMeshComponent.SetStaticMesh` _base_7 "/OpenXR/Devices/HPMixedReality/Left/left_HPMixedRealityController.left_HPMixedRealityController")
          (`PrimitiveComponent.CreateDynamicMaterialInstance` (`self.Base`) 0 "/CustomOpenXRControllerIntegration/Materials/HPMixedReality/M_XRController_HPMixedReality_Left.M_XRController_HPMixedReality_Left" "None")
          (goto _label_2)
          (else
            (`StaticMeshComponent.SetStaticMesh` (`self.Base`) "/OpenXR/Devices/MicrosoftMixedReality/Left/left_MicrosoftMixedRealityController.left_MicrosoftMixedRealityController")
            (`PrimitiveComponent.CreateDynamicMaterialInstance` (`self.Base`) 0 "/CustomOpenXRControllerIntegration/Materials/MicrosoftMixedReality/M_XRController_MicrosoftMixedReality.M_XRController_MicrosoftMixedReality" "None")
            (goto _label_2))))
      (:`DT_UnknownController`
        (goto _label_3)))
    (else
      (switch `EBPOpenXRControllerDeviceType` InputPin
        (:`DT_ValveIndexController`
          (`StaticMeshComponent.SetStaticMesh` _base_5 "/OpenXR/Devices/ValveIndex/Right/right_ValveIndexController.right_ValveIndexController")
          (`PrimitiveComponent.CreateDynamicMaterialInstance` (`self.Base`) 0 "/CustomOpenXRControllerIntegration/Materials/ValveIndex/MI_XRController_ValveIndex_Right.MI_XRController_ValveIndex_Right" "None")
          (`self.isChild Actor`
            (:`true`
              (`SceneComponent.K2_SetRelativeLocation` _base_5 (-5.0 2.0 -2.0) false true))))
        (:`DT_ViveController`
          (`StaticMeshComponent.SetStaticMesh` (`self.Base`) "/OpenXR/Devices/HTCVive/HTCViveController.HTCViveController" :!label _label_5)
          (`self.isChild Actor` :!label _label_6
            (:`true`
              (`SceneComponent.K2_SetRelativeLocation` _base_6 (-5.0 0.0 -2.0) false true))))
        (:`DT_ViveProController`
          (goto _label_5))
        (:`DT_OculusTouchController`
          (`self.GetOculusTouchVersion` InputPin2 :!label _label_7
            (:`Oculus Touch V2`
              (`StaticMeshComponent.SetStaticMesh` (`self.Base`) "/OpenXR/Devices/OculusTouch_v2/Right/right_OculusTouch_v2Controller.right_OculusTouch_v2Controller")
              (`PrimitiveComponent.CreateDynamicMaterialInstance` (`self.Base`) 0 "/CustomOpenXRControllerIntegration/Materials/OculusTouch_v2/MI_XRController_OculusTouch_v2_Right.MI_XRController_OculusTouch_v2_Right" "None")
              (`self.isChild Actor` :!label _label_8
                (:`true`
                  (`SceneComponent.K2_SetRelativeLocation` _base_2 (-5.0 0.0 0.0) false true))))
            (:`Oculus Touch V3`
              (`StaticMeshComponent.SetStaticMesh` _base "/OpenXR/Devices/OculusTouch_v3/Right/right_OculusTouch_v3Controller.right_OculusTouch_v3Controller")
              (`PrimitiveComponent.CreateDynamicMaterialInstance` (`self.Base`) 0 "/CustomOpenXRControllerIntegration/Materials/OculusTouch_v3/MI_XRController_OculusTouch_v3_Right.MI_XRController_OculusTouch_v3_Right" "None")
              (goto _label_8))
            (:`Oculus Touch V1`
              (`StaticMeshComponent.SetStaticMesh` _base "/OpenXR/Devices/OculusTouch/Right/right_OculusTouchController.right_OculusTouchController")
              (`PrimitiveComponent.CreateDynamicMaterialInstance` (`self.Base`) 0 "/CustomOpenXRControllerIntegration/Materials/OculusTouch/MI_XRController_OculusTouch_Right.MI_XRController_OculusTouch_Right" "None")
              (`self.isChild Actor`
                (:`true`
                  (`SceneComponent.K2_SetRelativeLocation` _base_2 (-5.0 0.0 -2.0) false true))))))
        (:`DT_MicrosoftMotionController`
          (if (`KismetStringLibrary.Contains` InputPin2 "Reverb G2" false true)
            (`StaticMeshComponent.SetStaticMesh` (`self.Base`) "/OpenXR/Devices/HPMixedReality/Right/right_HPMixedRealityController.right_HPMixedRealityController")
            (`PrimitiveComponent.CreateDynamicMaterialInstance` (`self.Base`) 0 "/CustomOpenXRControllerIntegration/Materials/HPMixedReality/M_XRController_HPMixedReality_Right.M_XRController_HPMixedReality_Right" "None")
            (goto _label_6)
            (else
              (`StaticMeshComponent.SetStaticMesh` _base_6 "/OpenXR/Devices/MicrosoftMixedReality/Right/right_MicrosoftMixedRealityController.right_MicrosoftMixedRealityController")
              (`PrimitiveComponent.CreateDynamicMaterialInstance` (`self.Base`) 0 "/CustomOpenXRControllerIntegration/Materials/MicrosoftMixedReality/M_XRController_MicrosoftMixedReality.M_XRController_MicrosoftMixedReality" "None")
              (goto _label_6))))
        (:`DT_UnknownController`
          (goto _label_7)))))
  (set `self.DefaultVector` (`SceneComponent.RelativeLocation` (`self.Base`))))

(fn `SpoofingControllers`
  (params (NameSystem :type String) (DeviceType :type "EBPOpenXRControllerDeviceType Enum" :default "DT_SimpleController"))
  (returns (ReturnValue :type "EBPOpenXRControllerDeviceType Enum") (ReturnValue2 :type String))
  (locals (NewLocalVar_0 :type "Array of String"))
  (bind _returnvalue (and (`self.SpoofController`) (not (`KismetSystemLibrary.IsPackagedForDistribution`))))
  (return (select `bool` _returnvalue :`false` DeviceType :`true` (`self.SpoofedControllerType`)) (select `bool` _returnvalue :`false` NameSystem :`true` (`|GetArrayItem` (`local.NewLocalVar_0`) (`self.EnumString`)))))

(fn `UserConstructionScript`
  (`parent.UserConstructionScript`))